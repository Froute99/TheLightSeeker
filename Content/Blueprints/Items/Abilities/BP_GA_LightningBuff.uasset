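; Gameplay ability that gives the player a timed lightning elemental buff.
; On activation it stores a lightning spread effect spec on the owning LightSeekerPlayerState as its elemental effect handle, rather than applying it directly, and applies a VFX holder effect to the owner.
; A ten-second delay task then ends the ability, and the end event clears the elemental effect from the player state.
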(event `self.K2_ActivateAbility`
  ;[1 1 1] Give EffectSpecHandle to Player
  (`parent.K2_ActivateAbility`)
  (bind _aslight_seeker_player_state (cast `LightSeekerPlayerState` (`.OwnerActor` (break `GameplayAbilityActorInfo` (`self.GetActorInfo`)))))
  (set `LightSeekerPlayerState.ElementalEffectHandle` (`self.MakeOutgoingGameplayEffectSpec` "/Game/Blueprints/Items/GameplayEffects/BP_GE_LightningSpreadHolder.BP_GE_LightningSpreadHolder_C") _aslight_seeker_player_state)
  (`KismetSystemLibrary.LogString` "Set PS Buff EffectHandle")
  ;[1 1 1] Apply VFX
  (`self.BP_ApplyGameplayEffectToOwner` "/Game/Blueprints/Items/GameplayEffects/BP_GE_LightningVFXHolder.BP_GE_LightningVFXHolder_C")
  (`AbilityTask_WaitDelay.WaitDelay` 10.0
    (:`OnFinish`
      (`self.K2_EndAbility`))))

(event `self.K2_OnEndAbility`
  (params (bWasCancelled :type Boolean))
  (bind _aslight_seeker_player_state (cast `LightSeekerPlayerState` (`.OwnerActor` (break `GameplayAbilityActorInfo` (`self.GetActorInfo`)))))
  (`LightSeekerPlayerState.ClearElementalEffect` _aslight_seeker_player_state))
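; Gameplay Cue notify actor that shows a freezing visual on enemies affected by an ice effect.
; OnActive casts the target to EnemyBase and sets the freezing material as its mesh overlay.
; OnRemove sets the overlay to a hardcoded green goblin material instead of clearing or restoring the previous one.
; Both handlers log when the target is not an enemy.
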(fn `OnActive`
  (params (MyTarget :type "Actor Object Reference") (Parameters :type "GameplayCueParameters Structure (by ref)"))
  (returns (ReturnValue :type Boolean))
  (`KismetSystemLibrary.LogString` "GC On Active")
  ;[1 1 1] Apply Material to target
  (bind _asenemy_base (cast `EnemyBase` MyTarget)
    (:`then`
      (`MeshComponent.SetOverlayMaterial` (`Character.Mesh` _asenemy_base) "/Game/Blueprints/Items/GameplayCues/M_Freezing.M_Freezing")
      (return false))
    (:`CastFailed`
      (`KismetSystemLibrary.LogString` "Target is not enemy"))))

(fn `OnRemove`
  (params (MyTarget :type "Actor Object Reference") (Parameters :type "GameplayCueParameters Structure (by ref)"))
  (returns (ReturnValue :type Boolean))
  ;[1 1 1] Apply Material to target
  (bind _asenemy_base (cast `EnemyBase` MyTarget)
    (:`then`
      (`MeshComponent.SetOverlayMaterial` (`Character.Mesh` _asenemy_base) "/Game/Goblin/Material/Goblin_Base/Mat_Goblin_green.Mat_Goblin_green")
      (return false))
    (:`CastFailed`
      (`KismetSystemLibrary.LogString` "Target is not enemy"))))

(fn `UserConstructionScript`)
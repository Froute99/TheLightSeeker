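; Enemy controller Blueprint that forwards damage events to the game mode to show floating damage text.
; On BeginPlay it calls BindDelegate and prints a message if binding fails.
; FloatingDamage takes the target ability system component's owner location and the damage value, then OnFloatingDamage casts the game mode to BP_TestGameMode and calls SpawnTextActor, printing a message if the cast fails.
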(event `Bind`
  (bind _returnvalue (`self.BindDelegate`))
  (if (not _returnvalue)
    (`KismetSystemLibrary.PrintString` "Bind failure")))

(event `self.ReceiveBeginPlay`
  (`self.Bind`))

(event `self.FloatingDamage`
  (params (SourceASC :type "CharacterAbilitySystemComponent Object Reference") (TargetASC :type "CharacterAbilitySystemComponent Object Reference") (Value :type "Float (single-precision)"))
  (`self.OnFloatingDamage` (`self.K2_GetActorLocation` (`ActorComponent.GetOwner` TargetASC)) Value))

(event `OnFloatingDamage`
  (params (Location :type "Vector Structure") (Damage :type "Float (double-precision)"))
  (bind _asbp_test_game_mode (cast `/Game/Blueprints/Core/BP_TestGameMode` (`GameplayStatics.GetGameMode`))
    (:`then`
      (`/Game/Blueprints/Core/BP_TestGameMode.SpawnTextActor` _asbp_test_game_mode Location Damage))
    (:`CastFailed`
      (`KismetSystemLibrary.PrintString` "Cast Failure to TestGameMode"))))

(fn `UserConstructionScript`)
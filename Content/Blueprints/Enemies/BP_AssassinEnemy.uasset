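; Assassin enemy Blueprint whose own graph only keeps its HP bar facing the player.
; Each tick it gets the pawn of player controller 0, casts it to CharacterBase and sets the HPBar world rotation to look from the enemy's location toward that character's camera.
; BeginPlay, overlap and the construction script are empty, so no combat or AI logic appears here.
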(event `self.ReceiveTick`
  (params (DeltaSeconds :type "Float (single-precision)"))
  (bind _returnvalue (`GameplayStatics.GetPlayerController` 0))
  ;[1 1 1] Update HPBar Rotation
  (if (`KismetSystemLibrary.IsValid` _returnvalue)
    (bind _ascharacter_base (cast `CharacterBase` (`Controller.K2_GetPawn` _returnvalue)))
    (`SceneComponent.K2_SetWorldRotation` (`self.HPBar`) (`KismetMathLibrary.FindLookAtRotation` (`self.K2_GetActorLocation`) (`SceneComponent.K2_GetComponentLocation` (`CharacterBase.Camera` _ascharacter_base))) false false)))

(fn `UserConstructionScript`)
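; Main character Blueprint that handles the skill tree toggle input and wires up references to HUD widgets.
; The IA_ToggleSkillTree Enhanced Input action calls ToggleWidget on the ACSkillTree component.
; RegisterWidgets takes a parent widget and caches its health bar, item and boss HP bar sub-widgets, and also assigns ACSkillTree to the SkillTreeComponent reference.
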(event `EnhancedInput|/Game/Blueprints/MainCharacter/Input/IA_ToggleSkillTree`
  (params (ActionValue :type Boolean) (ElapsedSeconds :type "Float (double-precision)") (TriggeredSeconds :type "Float (double-precision)") (InputAction :type "InputAction Object Reference" :default "/Game/Blueprints/MainCharacter/Input/IA_ToggleSkillTree.IA_ToggleSkillTree"))
  (:`Triggered`
    (`/Game/Blueprints/MainCharacter/AC_SkillTree.Toggle Widget` (`self.AC_SkillTree`))))

(fn `Register Widgets`
  (params (Widget :type "/Game/Blueprints/UI/WB_HUD Object Reference"))
  (set `self.HealthBar` (`/Game/Blueprints/UI/WB_HUD.WB_HealthBar` Widget))
  (set `self.ItemWidget` (`/Game/Blueprints/UI/WB_HUD.WB_ItemWidget` Widget))
  (set `self.SkillTreeComponent` (`self.AC_SkillTree`))
  (set `self.BossHPWidget` (`/Game/Blueprints/UI/WB_HUD.WB_BossEnemyHPBar` Widget)))

(fn `UserConstructionScript`)
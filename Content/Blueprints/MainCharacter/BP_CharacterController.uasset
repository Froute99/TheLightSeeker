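; Player controller Blueprint for the main character that relays damage events into floating damage text.
; FloatingDamage finds the damaged pawn's location through the target ability system component's owning LightSeekerPlayerState and passes it with the value to OnFloatingDamage.
; That event, logged as a send to the server, asks BP_TestGameMode to spawn the text actor.
; Debug prints trace the flow, and the delegate-binding logic is left unconnected.
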(event `Bind`)

(event `self.FloatingDamage`
  (params (SourceASC :type "CharacterAbilitySystemComponent Object Reference") (TargetASC :type "CharacterAbilitySystemComponent Object Reference") (Value :type "Float (single-precision)"))
  (`KismetSystemLibrary.PrintString` "PC: Event Triggered Floating Damage")
  (`self.OnFloatingDamage` (`self.K2_GetActorLocation` (`PlayerState.GetPawn` (cast `LightSeekerPlayerState` (`ActorComponent.GetOwner` TargetASC) :!pure true))) Value))

(event `OnFloatingDamage`
  (params (Location :type "Vector Structure") (Damage :type "Float (double-precision)"))
  (`KismetSystemLibrary.PrintString` "PC: Send Event to Server")
  (bind _asbp_test_game_mode (cast `/Game/Blueprints/Core/BP_TestGameMode` (`GameplayStatics.GetGameMode`))
    (:`then`
      (`/Game/Blueprints/Core/BP_TestGameMode.SpawnTextActor` _asbp_test_game_mode Location Damage))
    (:`CastFailed`
      (`KismetSystemLibrary.PrintString` "Cast Failure to TestGameMode"))))

(fn `UserConstructionScript`)
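; BP_Snipe is a homing projectile that applies a pierce-shot effect to an enemy.
; On BeginPlay it picks from all EnemyBase actors at random, with separate rolls for Target and the homing capsule, so the two can differ.
; Overlapping Target applies GE_PierceShot through the Instigator's ability system, prints the enemy's health and destroys the projectile; other overlaps are ignored.
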(event `self.ReceiveBeginPlay`
  (bind _outactors (`GameplayStatics.GetAllActorsOfClass` "/Script/TheLightSeeker.EnemyBase"))
  (bind _output (`|GetArrayItem` _outactors (`KismetMathLibrary.RandomInteger` (`KismetArrayLibrary.Array_Length` _outactors))))
  (set `self.Target` _output)
  (set `ProjectileMovementComponent.HomingTargetComponent` (`self.GetComponentByClass` _output "/Script/Engine.CapsuleComponent") (`self.ProjectileMovementComponent`))
  (`KismetSystemLibrary.PrintString` (`KismetSystemLibrary.GetDisplayName` _output)))

(event `self.ReceiveActorBeginOverlap`
  (params (OtherActor :type "Actor Object Reference"))
  (bind _returnvalue (`AbilitySystemBlueprintLibrary.GetAbilitySystemComponent` (`self.Target`)))
  (if (and (!= (`self.Instigator`) OtherActor) (== OtherActor (`self.Target`)))
    (`/Engine/EditorBlueprintResources/StandardMacros.IsValid` _returnvalue
      (:`Is Valid`
        (`AbilitySystemComponent.BP_ApplyGameplayEffectToTarget` :`self` (`AbilitySystemBlueprintLibrary.GetAbilitySystemComponent` (`self.Instigator`)) :`GameplayEffectClass` "/Game/Blueprints/Abilities/GE_PierceShot.GE_PierceShot_C" :`Target` _returnvalue)
        (bind _asenemy_base (cast `EnemyBase` (`self.Target`)))
        (`KismetSystemLibrary.PrintString` (`KismetStringLibrary.Conv_DoubleToString` (`EnemyBase.GetHealth` _asenemy_base)))
        (`self.K2_DestroyActor`))
      (:`Is Not Valid`
        (`KismetSystemLibrary.PrintString` "ASC not valid; from blueprint")))))

(fn `UserConstructionScript`)
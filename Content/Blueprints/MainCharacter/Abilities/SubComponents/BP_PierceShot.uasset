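; Pierce shot ability actor that applies a gameplay effect to each target it passes through, up to a limited count.
; On overlap with any non-instigator that has an ability system component, the instigator's component applies BP_GE_PierceShot to it and the Overlapping counter drops.
; For EnemyBase targets, it prints health for debugging and destroys itself once the counter runs out.
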(event `self.ReceiveActorBeginOverlap`
  (params (OtherActor :type "Actor Object Reference"))
  (bind _returnvalue (`AbilitySystemBlueprintLibrary.GetAbilitySystemComponent` OtherActor))
  (if (!= (`self.Instigator`) OtherActor)
    (`/Engine/EditorBlueprintResources/StandardMacros.IsValid` _returnvalue
      (:`Is Valid`
        (`AbilitySystemComponent.BP_ApplyGameplayEffectToTarget` :`self` (`AbilitySystemBlueprintLibrary.GetAbilitySystemComponent` (`self.Instigator`)) :`GameplayEffectClass` "/Game/Blueprints/MainCharacter/Abilities/GameplayEffect/BP_GE_PierceShot.BP_GE_PierceShot_C" :`Target` _returnvalue)
        (`/Engine/EditorBlueprintResources/StandardMacros.DecrementInt` (`self.Overlapping`)
          (:`  `
            (bind _asenemy_base (cast `EnemyBase` OtherActor))
            (`KismetSystemLibrary.PrintString` (`KismetStringLibrary.Conv_DoubleToString` (`EnemyBase.GetHealth` _asenemy_base)))
            (if (<= (`self.Overlapping`) 0)
              (`self.K2_DestroyActor`)
              (else
                (`KismetSystemLibrary.PrintString` (`KismetStringLibrary.Concat_StrStr` "PierceShot: " (`KismetStringLibrary.Conv_IntToString` (`self.Overlapping`)))))))))
      (:`Is Not Valid`
        (`KismetSystemLibrary.PrintString` "ASC not valid; from blueprint")))))

(fn `UserConstructionScript`)
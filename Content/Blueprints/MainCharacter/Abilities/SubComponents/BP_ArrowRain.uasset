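; BP_ArrowRain is an area ability actor for the main character that periodically damages enemies standing inside it.
; Begin and end overlap events maintain the Overlapped list, which a looping timer walks to apply the BP_GE_BasicAttack gameplay effect through each enemy's Ability System Component.
; Each hit is a random roll whose chance rises with enemy scale.
; After three seconds it stops the Niagara spawn rate, then destroys itself following a short delay.
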(event `self.ReceiveBeginPlay`
  (`KismetSystemLibrary.K2_SetTimerDelegate` (delegate `GiveDamage`) (`self.Interval`) true))

(event `GiveDamage`
  ;[1 1 1] Deal Damage
  (for _array_element (`self.Overlapped`)
    (bind _asenemy_base (cast `EnemyBase` _array_element))
    (if (<= (`KismetMathLibrary.RandomFloat`) (+ (/ (`EnemyBase.GetScale` _asenemy_base) 10.0) 0.6))
      (bind _returnvalue (`AbilitySystemBlueprintLibrary.GetAbilitySystemComponent` _asenemy_base))
      (`/Engine/EditorBlueprintResources/StandardMacros.IsValid` _returnvalue
        (:`Is Valid`
          (`AbilitySystemComponent.BP_ApplyGameplayEffectToSelf` :`self` _returnvalue :`GameplayEffectClass` "/Game/Blueprints/MainCharacter/Abilities/GameplayEffect/BP_GE_BasicAttack.BP_GE_BasicAttack_C")))))
  ;[1 1 1] Finishing Effect
  (if (>= (`self.GetGameTimeSinceCreation`) 3.0)
    (`NiagaraComponent.SetVariableFloat` (`self.Niagara`) "SpawnRate" 0.0)
    (`KismetSystemLibrary.Delay` 1.5)
    (`self.K2_DestroyActor`)))

(event `self.ReceiveActorBeginOverlap`
  (params (OtherActor :type "Actor Object Reference"))
  ;[1 1 1] Overlap
  (`KismetArrayLibrary.Array_Add` (`self.Overlapped`) OtherActor))

(event `self.ReceiveActorEndOverlap`
  (params (OtherActor :type "Actor Object Reference"))
  ;[1 1 1] Overlap
  (`KismetArrayLibrary.Array_RemoveItem` (`self.Overlapped`) OtherActor))

(fn `UserConstructionScript`)
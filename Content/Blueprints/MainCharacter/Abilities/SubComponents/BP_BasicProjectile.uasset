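; BP_BasicProjectile is an ability projectile that applies gameplay effects to actors it overlaps.
; On server overlap with a non-instigator that has an Ability System Component, the instigator's component applies the damage effect and an additional elemental effect spec.
; It destroys itself after affecting an EnemyBase or on any hit, while other affected actors let it continue.
; BeginPlay passes X and Y velocity to its Niagara effect.
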(event `self.ReceiveBeginPlay`
  (bind (_velocity_x _velocity_y) (`KismetMathLibrary.BreakVector` (`MovementComponent.Velocity` (`self.ProjectileMovementComponent`))))
  (`NiagaraComponent.SetVariableVec3` (`self.Niagara`) "Velocity" (`KismetMathLibrary.MakeVector` _velocity_x _velocity_y)))

(event `self.ReceiveActorBeginOverlap`
  (params (OtherActor :type "Actor Object Reference"))
  (bind _returnvalue (`AbilitySystemBlueprintLibrary.GetAbilitySystemComponent` OtherActor))
  (bind _returnvalue_2 (`AbilitySystemBlueprintLibrary.GetAbilitySystemComponent` (`self.Instigator`)))
  (`/Engine/EditorBlueprintResources/ActorMacros.Switch Has Authority`
    (:`Authority`
      (if (!= (`self.Instigator`) OtherActor)
        (`/Engine/EditorBlueprintResources/StandardMacros.IsValid` _returnvalue
          (:`Is Valid`
            (`AbilitySystemComponent.BP_ApplyGameplayEffectToTarget` :`self` _returnvalue_2 :`GameplayEffectClass` (`self.DamageEffect`) :`Target` _returnvalue)
            ;[1 1 1] Elemental effect
            (`AbilitySystemComponent.BP_ApplyGameplayEffectSpecToTarget` _returnvalue_2 (`self.AdditionalEffectSpecHandle`) _returnvalue)
            (cast `EnemyBase` OtherActor)
            (`self.K2_DestroyActor`))
          (:`Is Not Valid`
            (`KismetSystemLibrary.PrintString` "ASC not valid; from blueprint" true false)))))))

(event `self.ReceiveHit`
  (params (MyComp :type "PrimitiveComponent Object Reference") (Other :type "Actor Object Reference") (OtherComp :type "PrimitiveComponent Object Reference") (bSelfMoved :type Boolean) (HitLocation :type "Vector Structure") (HitNormal :type "Vector Structure") (NormalImpulse :type "Vector Structure") (Hit :type "HitResult Structure (by ref)"))
  (`self.K2_DestroyActor`))

(fn `UserConstructionScript`)
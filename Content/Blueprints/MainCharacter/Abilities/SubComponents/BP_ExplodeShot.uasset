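; BP_ExplodeShot is a main-character ability actor that acts as an exploding shot, triggered by overlapping any actor other than its Instigator.
; On overlap it runs a debug-drawn Pawn-profile sphere multi-trace around that actor's location, then destroys itself.
; For each non-Instigator hit, it applies BP_GE_BasicAttack through GetAbilitySystemComponent, which is called without the hit actor as input.
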(event `self.ReceiveActorBeginOverlap`
  (params (OtherActor :type "Actor Object Reference"))
  (bind _returnvalue (`AbilitySystemBlueprintLibrary.GetAbilitySystemComponent` null))
  (bind _returnvalue_2 (`self.K2_GetActorLocation` OtherActor))
  (if (!= OtherActor (`self.Instigator`))
    (bind _outhits (`KismetSystemLibrary.SphereTraceMultiByProfile` :`Start` _returnvalue_2 :`End` _returnvalue_2 :`Radius` 500.0 :`ProfileName` "Pawn" :`DrawDebugType` "ForDuration"))
    (for _array_element _outhits
      (if (and (!= (`.HitActor` (`GameplayStatics.BreakHitResult` _array_element)) (`self.Instigator`)) (`KismetSystemLibrary.IsValid` _returnvalue))
        (`AbilitySystemComponent.BP_ApplyGameplayEffectToSelf` :`self` _returnvalue :`GameplayEffectClass` "/Game/Blueprints/MainCharacter/Abilities/GameplayEffect/BP_GE_BasicAttack.BP_GE_BasicAttack_C")))
    (`self.K2_DestroyActor`)))

(fn `UserConstructionScript`)
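; BP_GA_MultiShot is the main character's multi-shot gameplay ability, which fires two arrows at once.
; On activation it calls PlayAnim, then spawns two ArrowClass actors at the avatar's location, always spawning regardless of collision, with the avatar pawn as instigator.
; Each arrow combines the avatar's rotation with an equal, opposite angular offset.
; The graph does not call CommitAbility or EndAbility.
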(event `self.K2_ActivateAbility`
  (bind _returnvalue (`self.GetAvatarActorFromActorInfo`))
  (bind _returnvalue_2 (`self.GetAvatarActorFromActorInfo`))
  (`self.PlayAnim`)
  (`|ExecutionSequence`
    (:`then_0`
      (`|SpawnActorFromClass` (`self.ArrowClass`) (`KismetMathLibrary.MakeTransform` (`Actor.K2_GetActorLocation` _returnvalue_2) (`KismetMathLibrary.ComposeRotators` (`Actor.K2_GetActorRotation` _returnvalue_2) (struct :`Yaw` 30.0))) "AlwaysSpawn" "MultiplyWithRoot" null (cast `Pawn` _returnvalue_2 :!pure true)))
    (:`then_1`
      (`|SpawnActorFromClass` (`self.ArrowClass`) (`KismetMathLibrary.MakeTransform` (`Actor.K2_GetActorLocation` _returnvalue) (`KismetMathLibrary.ComposeRotators` (`Actor.K2_GetActorRotation` _returnvalue) (struct :`Yaw` -30.0))) "AlwaysSpawn" "MultiplyWithRoot" null (cast `Pawn` _returnvalue :!pure true)))))
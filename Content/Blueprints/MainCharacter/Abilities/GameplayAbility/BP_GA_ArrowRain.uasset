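; Arrow Rain gameplay ability for the main character that places an area-of-effect at a targeted ground point.
; On activation it waits for user-confirmed target data from the BP_GA_GroundTrace target actor, with debug enabled.
; Confirming spawns BP_Test_AOE at that point, owned and instigated by the avatar, then ends; cancelling prints a "SnipeShot" debug message and ends.
; The animation call and EnemyBase target filter are unconnected.
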(event `self.K2_ActivateAbility`
  (bind _returnvalue (`self.GetAvatarActorFromActorInfo`))
  (bind (_asynctaskproxy _data) (`AbilityTask_WaitTargetData.WaitTargetData` "None" "UserConfirmed" "/Game/Blueprints/MainCharacter/Abilities/GameplayAbility/BP_GA_GroundTrace.BP_GA_GroundTrace_C" 0.0 0.0 999999.0 (struct :`Name` "BlockAllDynamic") true (`self.MakeTargetLocationInfoFromOwnerActor`) (struct) null (struct) true)
    (:`ValidData`
      (bind _returnvalue_location (`KismetMathLibrary.BreakTransform` (`AbilitySystemBlueprintLibrary.GetTargetDataEndPointTransform` _data)))
      (`|SpawnActorFromClass` "/Game/Blueprints/MainCharacter/Abilities/BP_Test_AOE.BP_Test_AOE_C" (`KismetMathLibrary.MakeTransform` _returnvalue_location) "AlwaysSpawn" "OverrideRootScale" _returnvalue (cast `Pawn` _returnvalue :!pure true))
      (`self.K2_EndAbility`))
    (:`Cancelled`
      (`KismetSystemLibrary.PrintString` "SnipeShot : Cancelled")
      (`self.K2_EndAbility`))))
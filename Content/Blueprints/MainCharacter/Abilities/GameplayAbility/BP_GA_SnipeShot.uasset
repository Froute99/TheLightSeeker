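; Gameplay ability for the main character's snipe shot, which fires a BP_Snipe actor at a player-confirmed enemy.
; On activation it waits for single-line-trace targeting with a reticle, filtered to EnemyBase actors.
; On confirm it plays an animation, spawns BP_Snipe at the avatar's transform with the first targeted actor as Target, then ends.
; Cancelling just ends the ability; targeting debug and log prints are enabled.
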(event `self.K2_ActivateAbility`
  (bind _returnvalue (`self.GetAvatarActorFromActorInfo`))
  (bind (_asynctaskproxy _data) (`AbilityTask_WaitTargetData.WaitTargetData` "None" "UserConfirmed" "/Script/GameplayAbilities.GameplayAbilityTargetActor_SingleLineTrace" 3000.0 (struct :`Name` "Pawn") true (`self.MakeTargetLocationInfoFromOwnerActor`) (struct) "/Game/Blueprints/MainCharacter/Abilities/BP_Reticle.BP_Reticle_C" (`AbilitySystemBlueprintLibrary.MakeFilterHandle` (make `GameplayTargetDataFilter` "/Script/TheLightSeeker.EnemyBase")) true)
    (:`ValidData`
      (`KismetSystemLibrary.PrintString` "SnipeShot : Ability targeting was confirmed")
      (`self.PlayAnim`)
      (`|SpawnActorFromClass` "/Game/Blueprints/MainCharacter/Abilities/BP_Snipe.BP_Snipe_C" (`Actor.GetTransform` _returnvalue) "AlwaysSpawn" "MultiplyWithRoot" _returnvalue (`|GetArrayItem` (`AbilitySystemBlueprintLibrary.GetActorsFromTargetData` _data)) (struct) (struct) (cast `Pawn` _returnvalue :!pure true))
      (`self.K2_EndAbility`))
    (:`Cancelled`
      (`KismetSystemLibrary.PrintString` "SnipeShot : Cancelled")
      (`self.K2_EndAbility`))))
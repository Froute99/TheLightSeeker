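; BP_AOE is a short-lived area-of-effect actor that periodically applies a gameplay effect, intended as damage, to pawns inside it.
; Overlap events maintain the list of actors in range, and a looping one-second timer applies the effect through each pawn's Ability System Component.
; After a few pulses it sets the Niagara spawn rate to zero and destroys itself following a short delay.
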(event `self.ReceiveActorBeginOverlap`
  (params (OtherActor :type "Actor Object Reference"))
  ;[1 1 1] Overlap
  (`KismetArrayLibrary.Array_Add` (`self.Overlapped`) OtherActor))

(event `self.ReceiveActorEndOverlap`
  (params (OtherActor :type "Actor Object Reference"))
  ;[1 1 1] Overlap
  (`KismetArrayLibrary.Array_RemoveItem` (`self.Overlapped`) OtherActor))

(event `self.ReceiveBeginPlay`
  (`KismetSystemLibrary.K2_SetTimerDelegate` (delegate `GiveDamage`) 1.0 true))

(event `GiveDamage`
  ;[1 1 1] Deal Damage
  (for _array_element (`self.Overlapped`)
    (bind _aspawn (cast `Pawn` _array_element))
    (bind _returnvalue (`AbilitySystemBlueprintLibrary.GetAbilitySystemComponent` _aspawn))
    (`/Engine/EditorBlueprintResources/StandardMacros.IsValid` _returnvalue
      (:`Is Valid`
        (`AbilitySystemComponent.BP_ApplyGameplayEffectToSelf` :`self` _returnvalue))))
  (bind _result (`/Engine/EditorBlueprintResources/StandardMacros.IncrementInt` (`self.TriggeredTimes`))
    (:`  `
      (if (== _result 3)
        (`NiagaraComponent.SetVariableFloat` (`self.Niagara`) "SpawnRate" 0.0)
        (`KismetSystemLibrary.Delay` 1.5)
        (`self.K2_DestroyActor`)))))

(fn `UserConstructionScript`)
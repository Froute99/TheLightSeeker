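; BP_Snipe is the homing projectile of the main character's snipe ability, fired at a preset Target.
; On BeginPlay it sets its projectile movement to home on the Target's capsule.
; It ignores overlaps with anything but that Target, then applies GE_SnipeShot through the Instigator's ability system.
; After applying the effect it prints the health and destroys itself, but only if the Target casts to EnemyBase.
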(event `self.ReceiveBeginPlay`
  (bind _target (`self.Target`)
    (:`then`
      (set `ProjectileMovementComponent.HomingTargetComponent` (`self.GetComponentByClass` _target "/Script/Engine.CapsuleComponent") (`self.ProjectileMovementComponent`)))
    (:`else`)))

(event `self.ReceiveActorBeginOverlap`
  (params (OtherActor :type "Actor Object Reference"))
  (bind _returnvalue (`AbilitySystemBlueprintLibrary.GetAbilitySystemComponent` (`self.Target`)))
  (if (and (!= (`self.Instigator`) OtherActor) (== OtherActor (`self.Target`)))
    (`/Engine/EditorBlueprintResources/StandardMacros.IsValid` _returnvalue
      (:`Is Valid`
        (`AbilitySystemComponent.BP_ApplyGameplayEffectToTarget` :`self` (`AbilitySystemBlueprintLibrary.GetAbilitySystemComponent` (`self.Instigator`)) :`GameplayEffectClass` "/Game/Blueprints/MainCharacter/Abilities/GameplayEffect/GE_SnipeShot.GE_SnipeShot_C" :`Target` _returnvalue)
        (bind _asenemy_base (cast `EnemyBase` (`self.Target`)))
        (`KismetSystemLibrary.PrintString` (`KismetStringLibrary.Conv_DoubleToString` (`EnemyBase.GetHealth` _asenemy_base)))
        (`self.K2_DestroyActor`)))))

(fn `UserConstructionScript`)
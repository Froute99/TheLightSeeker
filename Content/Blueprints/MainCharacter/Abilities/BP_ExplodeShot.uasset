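; BP_ExplodeShot is an exploding shot actor for a main character ability that deals area damage on overlap.
; Overlapping any actor except its Instigator runs a multi sphere trace on the Pawn profile around that actor's location, with debug drawing enabled.
; Each hit with an Ability System Component receives GE_Damage, with no Instigator filter on the hits, then the shot destroys itself.
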(event `self.ReceiveActorBeginOverlap`
  (params (OtherActor :type "Actor Object Reference"))
  (bind _returnvalue (`self.K2_GetActorLocation` OtherActor))
  (if (!= OtherActor (`self.Instigator`))
    (bind _outhits (`KismetSystemLibrary.SphereTraceMultiByProfile` :`Start` _returnvalue :`End` _returnvalue :`Radius` 500.0 :`ProfileName` "Pawn" :`DrawDebugType` "ForDuration"))
    (for _array_element _outhits
      (bind _returnvalue_2 (`AbilitySystemBlueprintLibrary.GetAbilitySystemComponent` (`.HitActor` (`GameplayStatics.BreakHitResult` _array_element))))
      (`/Engine/EditorBlueprintResources/StandardMacros.IsValid` _returnvalue_2
        (:`Is Valid`
          (`AbilitySystemComponent.BP_ApplyGameplayEffectToSelf` :`self` _returnvalue_2 :`GameplayEffectClass` "/Game/Blueprints/MainCharacter/Abilities/GameplayEffect/GE_Damage.GE_Damage_C"))))
    (`self.K2_DestroyActor`)))

(fn `UserConstructionScript`)
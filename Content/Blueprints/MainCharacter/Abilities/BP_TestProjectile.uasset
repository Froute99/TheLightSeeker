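; Test ability projectile for the main character that delivers Gameplay Ability System effects on hit.
; On box overlap, it applies its damage spec and an additional elemental-enchant spec to the other actor's Ability System Component.
; It destroys itself only if that actor is also an EnemyBase, printing its health first.
; Other cases just print debug messages, and a leftover elemental-handle failure log is never run.
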(event `self.BoxComponent.OnComponentBeginOverlap`
  (params (OverlappedComponent :type "PrimitiveComponent Object Reference") (OtherActor :type "Actor Object Reference") (OtherComp :type "PrimitiveComponent Object Reference") (OtherBodyIndex :type Integer) (bFromSweep :type Boolean) (SweepResult :type "HitResult Structure (by ref)"))
  (bind _returnvalue (`AbilitySystemBlueprintLibrary.GetAbilitySystemComponent` OtherActor))
  (`/Engine/EditorBlueprintResources/StandardMacros.IsValid` _returnvalue
    (:`Is Valid`
      (`AbilitySystemComponent.BP_ApplyGameplayEffectSpecToSelf` _returnvalue (`self.DamageEffectSpecHandle`))
      ;[1 1 1] Applying Additional Effect Added by Elemental Enchants
      (`AbilitySystemComponent.BP_ApplyGameplayEffectSpecToSelf` _returnvalue (`self.AdditionalEffectSpecHandle`))
      (bind _asenemy_base (cast `EnemyBase` OtherActor)
        (:`then`
          (`KismetSystemLibrary.PrintString` (`KismetStringLibrary.Conv_DoubleToString` (`EnemyBase.GetHealth` _asenemy_base)))
          (`self.K2_DestroyActor`))
        (:`CastFailed`
          (`KismetSystemLibrary.PrintString` "Overlapped actor is not a kind of enemybase"))))
    (:`Is Not Valid`
      (`KismetSystemLibrary.PrintString` "ASC not valid; from blueprint"))))

(fn `UserConstructionScript`)
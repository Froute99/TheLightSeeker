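; Basic ability projectile for the main character that damages whatever it overlaps through the Gameplay Ability System.
; On overlap with an actor other than its Instigator, the Instigator's ability system component applies GE_Damage to that actor, then the projectile destroys itself.
; Targets without an ability system component only print a debug message.
; An unconnected branch holds spec-handle damage with elemental enchant effects and enemy health printing; the box overlap event is empty.
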(event `self.ReceiveActorBeginOverlap`
  (params (OtherActor :type "Actor Object Reference"))
  (bind _returnvalue (`AbilitySystemBlueprintLibrary.GetAbilitySystemComponent` OtherActor))
  (if (!= (`self.Instigator`) OtherActor)
    (`/Engine/EditorBlueprintResources/StandardMacros.IsValid` _returnvalue
      (:`Is Valid`
        (`AbilitySystemComponent.BP_ApplyGameplayEffectToTarget` :`self` (`AbilitySystemBlueprintLibrary.GetAbilitySystemComponent` (`self.Instigator`)) :`GameplayEffectClass` "/Game/Blueprints/MainCharacter/Abilities/GameplayEffect/GE_Damage.GE_Damage_C" :`Target` _returnvalue)
        (`self.K2_DestroyActor`))
      (:`Is Not Valid`
        (`KismetSystemLibrary.PrintString` "ASC not valid; from blueprint")))))

(event `self.BoxComponent.OnComponentBeginOverlap`
  (params (OverlappedComponent :type "PrimitiveComponent Object Reference") (OtherActor :type "Actor Object Reference") (OtherComp :type "PrimitiveComponent Object Reference") (OtherBodyIndex :type Integer) (bFromSweep :type Boolean) (SweepResult :type "HitResult Structure (by ref)")))

(fn `UserConstructionScript`)
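; AC_SkillTree is an actor component on the player character that opens and closes the skill tree UI.
; BeginPlay caches the owning CharacterBase and its PlayerController.
; Toggle Widget either creates WB_SkillTree, adds it to the viewport, switches to UI-only input and shows the cursor, or removes the widget and restores game-only input with the cursor hidden.
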(event `self.ReceiveBeginPlay`
  (bind _ascharacter_base (cast `CharacterBase` (`self.GetOwner`)))
  (bind _output_get (set `self.Player` _ascharacter_base))
  (bind _asplayer_controller (cast `PlayerController` (`Pawn.GetController` _output_get)))
  (set `self.PlayerController` _asplayer_controller))

(fn `Toggle Widget`
  (bind _playercontroller (`self.PlayerController`))
  (bind _playercontroller_2 (`self.PlayerController`))
  (bind _wb_skilltree (`self.WB_SkillTree`)
    (:`then`
      (`Widget.RemoveFromParent` _wb_skilltree)
      (set `self.WB_SkillTree` null)
      (`WidgetBlueprintLibrary.SetInputMode_GameOnly` _playercontroller_2)
      (set `PlayerController.bShowMouseCursor` false _playercontroller_2))
    (:`else`
      (bind _returnvalue (`|CreateWidget` "/Game/Blueprints/UI/WB_SkillTree.WB_SkillTree_C" (`self.PlayerController`)))
      (bind _output_get (set `self.WB_SkillTree` _returnvalue))
      (`UserWidget.AddToViewport` _output_get 0)
      (`WidgetBlueprintLibrary.SetInputMode_UIOnlyEx` _playercontroller (`self.WB_SkillTree`))
      (set `PlayerController.bShowMouseCursor` true _playercontroller))))
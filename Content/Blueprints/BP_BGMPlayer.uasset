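; Background music player that switches between peaceful, combat and finish tracks as the fight progresses.
; On BeginPlay it binds to EnemySpawnManager's combat status and boss defeated delegates, which choose the next track, with combat updates ignoring an unchanged status.
; A single AudioComponent fades out, then a one-shot timer of the same duration swaps the sound and fades it back in.
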(event `self.ReceiveBeginPlay`
  (bind _enemyspawnmanager (`self.EnemySpawnManager`))
  (add `EnemySpawnManager.OnCombatStatusChangedDelegateHandle` _enemyspawnmanager (delegate `OnCombatStatusChanged`))
  (add `EnemySpawnManager.IsBossDefeatedDelegateHandle` _enemyspawnmanager (delegate `OnBossDefeated`)))

(event `OnBossDefeated`
  (bind _fadeoutduration (`self.FadeOutDuration`))
  (set `self.NextBGM` (`self.FinishBGM`))
  (`AudioComponent.FadeOut` (`self.AudioComponent`) _fadeoutduration 0.0 "Linear")
  (`KismetSystemLibrary.K2_SetTimerDelegate` (delegate `OnBGMFinished`) _fadeoutduration))

(event `OnCombatStatusChanged`
  (params (IsInCombat :type Boolean))
  (bind _fadeoutduration (`self.FadeOutDuration`))
  ;[1 1 1] Ignore if already in status
  (if (!= IsInCombat (`self.IsInCombat`))
    (bind _output_get (set `self.IsInCombat` IsInCombat))
    (if _output_get
      (set `self.NextBGM` (`self.CombatBGM`))
      (else
        (set `self.NextBGM` (`self.PeacefulBGM`))))
    ;[1 1 1] Play new BGM after fading out
    (`AudioComponent.FadeOut` (`self.AudioComponent`) _fadeoutduration 0.0 "Linear")
    (`KismetSystemLibrary.K2_SetTimerDelegate` (delegate `OnBGMFinished`) _fadeoutduration)))

(event `OnBGMFinished`
  (bind _audiocomponent (`self.AudioComponent`))
  ;[1 1 1] Helper to play BGM after original BGM finished
  (`AudioComponent.SetSound` _audiocomponent (`self.NextBGM`))
  (`AudioComponent.Play` _audiocomponent 0.0)
  (`AudioComponent.FadeIn` _audiocomponent (`self.FadeOutDuration`) 1.0 0.0 "Linear"))

(fn `UserConstructionScript`)
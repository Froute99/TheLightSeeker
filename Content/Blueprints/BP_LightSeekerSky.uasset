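; BP_LightSeekerSky is a sky Blueprint that changes the sky and sun lighting for the finale once the boss is defeated.
; On BeginPlay, only the authority binds to the EnemySpawnManager's boss-defeated delegate.
; That callback runs ChangeLightSettingForFinale, which assigns zenith, cloud, horizon and overall colors, recolors the Sun's light and refreshes the sky material.
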(event `self.ReceiveBeginPlay`
  (`/Engine/EditorBlueprintResources/ActorMacros.Switch Has Authority`
    (:`Authority`
      (add `EnemySpawnManager.IsBossDefeatedDelegateHandle` (`self.EnemySpawnManager`) (delegate `OnBossDefeated`)))))

(event `OnBossDefeated`
  (`self.ChangeLightSettingForFinale`))

(event `ChangeLightSettingForFinale`
  (set `self.Zenith Color` (`self.ZenithColor`))
  (set `self.Cloud color` (`self.CouldColor`))
  (set `self.Horizon color` (`self.HorizonColor`))
  (set `self.Overall Color` (`self.OverallColor`))
  (`LightComponent.SetLightColor` (`Light.LightComponent` (`self.Sun`)) (`self.SunColor`) true)
  (`self.RefreshMaterial`))

(fn `UserConstructionScript`
  (`parent.UserConstructionScript`))